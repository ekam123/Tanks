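; Toon Tanks game mode that sets up players and drives the start and end screens of a match.
; On BeginPlay it reads the players and five-player spawn locations from the BP_StoreVars game instance and passes them to SetPlayers.
; StartGame shows the start and player stats widgets.
; GameOver shows the end widget with win or lose text, which immediately overwrites its "Game Over" text.
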(event EventBeginPlay
  (Utilities|Casting|CastToBP_ToonTanksGameMode (Game|GetGameMode))
  (bind _asbp_store_vars (Utilities|Casting|CastToBP_StoreVars (Game|GetGameInstance)))
  (Class|ToonTanksGameMode|SetPlayers (Variables|/Game/Blueprints/BP_StoreVars.BP_StoreVars_C|GetGIPlayers _asbp_store_vars) (Variables|/Game/Blueprints/BP_StoreVars.BP_StoreVars_C|GetFivePlayerLocations _asbp_store_vars)))

(event EventTick
  (params (DeltaSeconds :type Float%20%28single-precision%29)))

(event EventStartGame
  (bind _returnvalue (UserInterface|CreateWidget "/Game/Blueprints/Widgets/WBP_StartGameWidget.WBP_StartGameWidget_C"))
  (UserInterface|Viewport|AddtoViewport _returnvalue 0)
  (bind _returnvalue_2 (UserInterface|CreateWidget "/Game/Blueprints/Widgets/WBP_PlayerStats.WBP_PlayerStats_C"))
  (UserInterface|Viewport|AddtoViewport _returnvalue_2 0))

(event EventGameOver
  (params (bWonGame :type Boolean))
  (bind _returnvalue (UserInterface|CreateWidget "/Game/Blueprints/Widgets/WBP_EndGameWidget.WBP_EndGameWidget_C"))
  (UserInterface|Viewport|AddtoViewport _returnvalue 0)
  (Rendering|Components|TextRender|SetText (Variables|/Game/Blueprints/Widgets/WBP_EndGameWidget.WBP_EndGameWidget_C|GetDisplayText _returnvalue) "Game Over")
  (Rendering|Components|TextRender|SetText (Variables|/Game/Blueprints/Widgets/WBP_EndGameWidget.WBP_EndGameWidget_C|GetDisplayText _returnvalue) (select bWonGame "You Won!" "You Lost!")))

(fn ConstructionScript)