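; BP_WheeledTank is a player-drivable wheeled tank vehicle in the Chaos Blueprints folder.
; MoveForward feeds throttle and inverted brake input to the vehicle movement component, while Turn steers through its yaw input rather than a steering input.
; Separate look axes drive controller yaw and inverted pitch.
; BeginPlay prints the mesh's gravity and physics simulation states for debugging.
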(event EventBeginPlay
  (bind _mesh (Variables|Character|GetMesh))
  (Development|PrintString (Utilities|String|ToString(Boolean) (Class|PrimitiveComponent|IsGravityEnabled _mesh)) true true "(R=0.000000,G=0.660000,B=1.000000,A=1.000000)" 5.0)
  (Development|PrintString (Utilities|String|ToString(Boolean) (Class|SceneComponent|IsAnySimulatingPhysics _mesh)) true true "(R=1.000000,G=0.257771,B=0.178056,A=1.000000)" 5.0))

(event Collision|EventActorBeginOverlap
  (params (OtherActor :type Actor%20Object%20Reference)))

(event EventTick
  (params (DeltaSeconds :type Float%20%28single-precision%29)))

(event Input|AxisEvents|InputAxisTurnRight/Left
  (params (AxisValue :type Float%20%28single-precision%29))
  (Pawn|Input|AddControllerYawInput AxisValue))

(event Input|AxisEvents|InputAxisMoveForward
  (params (AxisValue :type Float%20%28single-precision%29))
  (bind _vehiclemovementcomponent (Variables|Default|GetVehicleMovementComponent))
  (Class|ChaosVehicleMovementComponent|SetThrottleInput _vehiclemovementcomponent AxisValue)
  (Class|ChaosVehicleMovementComponent|SetBrakeInput _vehiclemovementcomponent (* AxisValue -1.0)))

(event Input|AxisEvents|InputAxisLookUp/Down
  (params (AxisValue :type Float%20%28single-precision%29))
  (Pawn|Input|AddControllerPitchInput (* AxisValue -1.0)))

(event Input|AxisEvents|InputAxisTurn
  (params (AxisValue :type Float%20%28single-precision%29))
  (Class|ChaosVehicleMovementComponent|SetYawInput (Variables|Default|GetVehicleMovementComponent) AxisValue))

(fn ConstructionScript)